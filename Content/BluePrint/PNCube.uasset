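; PNCube is an actor that tilts to match the surface beneath it.
; Each tick, Raycast traces 100 units along the actor's local down axis on the Visibility channel.
; On a hit, it aligns its up axis to the impact normal with MakeRotFromZX, using its forward vector as reference; otherwise JointSet restores world up.
; Fall and upward-movement logic is present but never runs.
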(event `self.ReceiveTick`
  (params (DeltaSeconds :type "Float (single-precision)"))
  (bind _returnvalue (`self.K2_GetActorLocation`))
  (bind _outhit (`KismetSystemLibrary.LineTraceSingle` _returnvalue (+ _returnvalue (* (`self.GetActorUpVector`) -100.0)) "TraceTypeQuery1"))
  (bind (_bblockinghit _binitialoverlap _time _distance _location _impactpoint _normal _impactnormal) (`GameplayStatics.BreakHitResult` _outhit))
  (if _bblockinghit
    (`self.K2_SetActorRotation` (`KismetMathLibrary.MakeRotFromZX` _impactnormal (`self.GetActorForwardVector`)))
    (else
      (`self.K2_SetActorRotation` (`KismetMathLibrary.MakeRotFromZX` (`KismetMathLibrary.MakeVector` 0.0 0.0 1.0) (`self.GetActorForwardVector`))))))

(fn `UserConstructionScript`)